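; Armed enemy character that wanders randomly and attacks the player character with a rifle on sight.
; PawnSensing triggers a chase via AIMoveTo, smoothly aiming ahead of the target using its velocity before firing.
; A timer, renewed by each sighting, exits combat when contact is lost, swapping weapon and lowering walk speed.
; Taking damage also reduces walk speed.
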(event `self.ReceiveAnyDamage`
  (params (Damage :type "Float (single-precision)") (DamageType :type "DamageType Object Reference") (InstigatedBy :type "Controller Object Reference") (DamageCauser :type "Actor Object Reference"))
  (bind _charactermovement (`self.CharacterMovement`))
  (`parent.ReceiveAnyDamage` Damage DamageType InstigatedBy DamageCauser)
  (set `CharacterMovementComponent.MaxWalkSpeed` (* (`CharacterMovementComponent.MaxWalkSpeed` _charactermovement) 0.8) _charactermovement)
  (`KismetSystemLibrary.Delay` 0.2))

(event `self.ReceiveBeginPlay`
  (`parent.ReceiveBeginPlay`)
  (`self.Vagar`))

(event `Vagar`
  ;[1 1 1] Vagar
  (if (`self.Muerto`)
    _
    (elif (not (`self.EnCombate`))
      (set `CharacterMovementComponent.bOrientRotationToMovement` true (`self.CharacterMovement`))
      (`|AIMoveTo` self (`NavigationSystemV1.K2_GetRandomReachablePointInRadius` (`self.K2_GetActorLocation`) 2000.0 null null) null 300.0
        (:`OnSuccess`
          _)
        (:`OnFail`
          _))
      (`KismetSystemLibrary.K2_SetTimerDelegate` (delegate `Vagar`) 4.0 true))))

(event `Salir_de_combate`
  ;[1 1 1] Persecución
  (set `self.EnCombate` false)
  (`self.Cambiar_arma` (`self.Arma`))
  (set `CharacterMovementComponent.MaxWalkSpeed` 300.0 (`self.CharacterMovement`))
  (set `self.apuntar_offset` (`KismetMathLibrary.RInterpTo` (`self.apuntar_offset`) (`KismetMathLibrary.MakeRotator` 0.0) (`GameplayStatics.GetWorldDeltaSeconds`) 10.0)))

(event `self.PawnSensing.OnSeePawn`
  (params (Pawn :type "Pawn Object Reference"))
  ;[1 1 1] Persecución
  (if (not (`self.Muerto`))
    (cast `/Game/Blueprints/Blueprints/ThirdPersonCharacter` Pawn)
    (`self.Persecucion` Pawn)))

(event `Persecucion`
  (params (Objetivo :type "Actor Object Reference"))
  (bind (_returnvalue_roll _returnvalue_pitch _returnvalue_yaw) (`KismetMathLibrary.BreakRotator` (`KismetMathLibrary.RInterpTo` (`self.Get absolute aim`) (`KismetMathLibrary.FindLookAtRotation` (`self.K2_GetActorLocation`) (+ (`self.K2_GetActorLocation` Objetivo) (/ (`self.GetVelocity` Objetivo) 2.0))) (`GameplayStatics.GetWorldDeltaSeconds`) 11.0)))
  ;[1 1 1] Persecución
  (if (`self.EnCombate`)
    (`KismetSystemLibrary.K2_ClearTimer` self "Salir_de_combate")
    (else
      (`self.Iniciar_combate`)))
  (`|AIMoveTo` self (0.0 0.0 0.0) Objetivo 3000.0
    (:`OnSuccess`
      _)
    (:`OnFail`
      _))
  (`self.Set absolute aim` (`KismetMathLibrary.MakeRotator` _returnvalue_roll _returnvalue_pitch _returnvalue_yaw))
  (`self.Ataque Rifle` null)
  (`KismetSystemLibrary.K2_SetTimer` self "Salir_de_combate" 1.0))

(event `Iniciar_combate`
  ;[1 1 1] Persecución
  (set `self.EnCombate` true)
  (set `CharacterMovementComponent.MaxWalkSpeed` 500.0 (`self.CharacterMovement`))
  (`self.Cambiar_arma` (`self.Arma`) "NewEnumerator1"))

(fn `UserConstructionScript`
  (`parent.UserConstructionScript`))