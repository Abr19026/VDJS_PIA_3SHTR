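; Player controller that handles the death screen, victory screen and respawn requests.
; On possess it binds to the pawn's OnDestroyed to trigger the game-over screen.
; Both screens create a widget and switch to UI-only input with the cursor shown.
; PedirRespawn forwards the load-save argument to the game mode, then, if the stored death widget is valid, removes it and restores game-only input.
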(event `self.ReceivePossess`
  (params (PossessedPawn :type "Pawn Object Reference"))
  (add `self.OnDestroyed` PossessedPawn (delegate `Accion_jugador_muere`)))

(event `Accion_jugador_muere` :!signature `self.OnDestroyed`
  (params (DestroyedActor :type "Actor Object Reference"))
  (`self.mostrar_pantalla_fin_juego`))

(event `mostrar_pantalla_fin_juego`
  (bind _returnvalue (`|CreateWidget` "/Game/Blueprints/Blueprints/GUI/GUI_muerte.GUI_muerte_C"))
  (bind _output_get (set `self.Widget_ult` _returnvalue))
  (`UserWidget.AddToViewport` _output_get 0)
  (`WidgetBlueprintLibrary.SetInputMode_UIOnlyEx` self null)
  (set `self.bShowMouseCursor` true))

(event `Mostrar_pantalla_victoria`
  (bind _returnvalue (`|CreateWidget` "/Game/Blueprints/Blueprints/GUI/GUI_victoria.GUI_victoria_C"))
  (`UserWidget.AddToViewport` _returnvalue 0)
  (`WidgetBlueprintLibrary.SetInputMode_UIOnlyEx` self null)
  (set `self.bShowMouseCursor` true))

(event `/Game/Blueprints/Blueprints/Datos_juego/interfaces/BPI_pedir_respawn.Pedir Respawn`
  (params (cargar_guardado :type Boolean))
  (bind _widget_ult (`self.Widget_ult`))
  (message `/Game/Blueprints/Blueprints/Datos_juego/interfaces/BPI_pedir_respawn.Pedir Respawn` (`GameplayStatics.GetGameMode`) cargar_guardado)
  (`/Engine/EditorBlueprintResources/StandardMacros.IsValid` _widget_ult
    (:`Is Valid`
      (`Widget.RemoveFromParent` _widget_ult)
      (`WidgetBlueprintLibrary.SetInputMode_GameOnly` self)
      (set `self.bShowMouseCursor` false))))

(fn `UserConstructionScript`)