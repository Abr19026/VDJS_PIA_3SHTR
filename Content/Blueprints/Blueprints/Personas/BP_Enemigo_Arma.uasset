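; Armed enemy character that wanders to random reachable points until PawnSensing spots a player character, then chases and fires a rifle.
; Combat switches weapon and speed, moves toward the target, and aims at its body or eye point with velocity-based lead, smoothed in Tick.
; A one-second timer, cleared on renewed pursuit, exits combat; taking damage cuts walk speed.
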(event `self.ReceiveAnyDamage`
  (params (Damage :type "Float (single-precision)") (DamageType :type "DamageType Object Reference") (InstigatedBy :type "Controller Object Reference") (DamageCauser :type "Actor Object Reference"))
  (bind _charactermovement (`self.CharacterMovement`))
  (`parent.ReceiveAnyDamage` Damage DamageType InstigatedBy DamageCauser)
  (set `CharacterMovementComponent.MaxWalkSpeed` (* (`CharacterMovementComponent.MaxWalkSpeed` _charactermovement) 0.8) _charactermovement)
  (`KismetSystemLibrary.Delay` 0.2))

(event `self.ReceiveBeginPlay`
  (`parent.ReceiveBeginPlay`)
  (`self.Vagar`))

(event `self.ReceiveTick`
  (params (DeltaSeconds :type "Float (single-precision)"))
  (bind (_apuntar_offset_roll _apuntar_offset_pitch) (`KismetMathLibrary.BreakRotator` (`self.apuntar_offset`)))
  (if (`self.rotando`)
    (`self.Set absolute aim` (`KismetMathLibrary.RInterpTo` (`self.Get absolute aim`) (`self.Rotacion_objetivo`) DeltaSeconds 4.0))
    (else
      (set `self.apuntar_offset` (`KismetMathLibrary.MakeRotator` 0.0 (`KismetMathLibrary.FInterpTo` _apuntar_offset_pitch 0.0 DeltaSeconds 4.0))))))

(event `Vagar`
  ;[1 1 1] Vagar
  (if (`self.Muerto`)
    _
    (elif (not (`self.EnCombate`))
      (set `CharacterMovementComponent.bOrientRotationToMovement` true (`self.CharacterMovement`))
      (`|AIMoveTo` self (`NavigationSystemV1.K2_GetRandomReachablePointInRadius` (`self.K2_GetActorLocation`) 2000.0 null null) null 300.0
        (:`OnSuccess`
          _)
        (:`OnFail`
          _))
      (`KismetSystemLibrary.K2_SetTimerDelegate` (delegate `Vagar`) 4.0 true))))

(event `Salir_de_combate`
  ;[1 1 1] Persecución
  (set `self.EnCombate` false)
  (`self.Cambiar_arma` (`self.Arma`))
  (set `CharacterMovementComponent.MaxWalkSpeed` 300.0 (`self.CharacterMovement`))
  (set `self.rotando` false))

(event `self.PawnSensing.OnSeePawn`
  (params (Pawn :type "Pawn Object Reference"))
  ;[1 1 1] Persecución
  (if (not (`self.Muerto`))
    (cast `/Game/Blueprints/Blueprints/Personas/ThirdPersonCharacter` Pawn)
    (`self.Persecucion` Pawn)))

(event `Persecucion`
  (params (Objetivo :type "Actor Object Reference"))
  ;[1 1 1] Persecución
  (if (`self.EnCombate`)
    (`KismetSystemLibrary.K2_ClearTimer` self "Salir_de_combate")
    (else
      (`self.Iniciar_combate`)))
  (`|AIMoveTo` self (0.0 0.0 0.0) Objetivo 3000.0 true
    (:`OnSuccess`
      _)
    (:`OnFail`
      _))
  (set `self.disparar_objetivo` (`KismetArrayLibrary.Array_Random` (`|MakeArray` (`self.K2_GetActorLocation` Objetivo) (`self.GetActorEyesViewPoint` Objetivo))))
  (set `self.Rotacion_objetivo` (`KismetMathLibrary.FindLookAtRotation` (`self.GetActorEyesViewPoint`) (+ (`self.disparar_objetivo`) (/ (`self.GetVelocity` Objetivo) 2.0))))
  (set `self.rotando` true)
  (`self.Ataque Rifle` null)
  (`KismetSystemLibrary.K2_SetTimer` self "Salir_de_combate" 1.0))

(event `Iniciar_combate`
  ;[1 1 1] Persecución
  (set `self.EnCombate` true)
  (set `CharacterMovementComponent.MaxWalkSpeed` 500.0 (`self.CharacterMovement`))
  (`self.Cambiar_arma` (`self.Arma`) "NewEnumerator1"))

(fn `UserConstructionScript`
  (`parent.UserConstructionScript`))