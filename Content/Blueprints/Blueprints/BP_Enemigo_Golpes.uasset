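; Melee enemy Blueprint that wanders at random, then chases and strikes the player character, building on a parent class.
; Vagar moves it to random reachable points on a repeating timer while it is alive and out of combat.
; PawnSensing sightings of a living ThirdPersonCharacter start Persecucion, a faster AIMoveTo chase that calls GolpeAtaque on arrival, then clears combat and resets speed.
; Taking damage runs parent handling and cuts current walk speed.
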(event `self.ReceiveAnyDamage`
  (params (Damage :type "Float (single-precision)") (DamageType :type "DamageType Object Reference") (InstigatedBy :type "Controller Object Reference") (DamageCauser :type "Actor Object Reference"))
  (bind _charactermovement (`self.CharacterMovement`))
  (`parent.ReceiveAnyDamage` Damage DamageType InstigatedBy DamageCauser)
  (set `CharacterMovementComponent.MaxWalkSpeed` (* (`CharacterMovementComponent.MaxWalkSpeed` _charactermovement) 0.8) _charactermovement)
  (`KismetSystemLibrary.Delay` 0.2))

(event `self.ReceiveBeginPlay`
  (`parent.ReceiveBeginPlay`)
  (`self.Vagar`))

(event `Vagar`
  ;[1 1 1] Vagar
  (if (`self.Muerto`)
    _
    (elif (not (`self.EnCombate`))
      (set `CharacterMovementComponent.bOrientRotationToMovement` true (`self.CharacterMovement`))
      (`|AIMoveTo` self (`NavigationSystemV1.K2_GetRandomReachablePointInRadius` (`self.K2_GetActorLocation`) 2000.0 null null) null 300.0
        (:`OnSuccess`
          _)
        (:`OnFail`
          _))
      (`KismetSystemLibrary.K2_SetTimerDelegate` (delegate `Vagar`) 4.0 true))))

(event `self.PawnSensing.OnSeePawn`
  (params (Pawn :type "Pawn Object Reference"))
  ;[1 1 1] Persecución
  (if (`self.Muerto`)
    _
    (elif (not (`self.EnCombate`))
      (bind _asthird_person_character (cast `/Game/Blueprints/Blueprints/ThirdPersonCharacter` Pawn))
      (if (not (`/Game/Blueprints/Blueprints/BP_Persona.Muerto` _asthird_person_character))
        (`self.Persecucion` Pawn)))))

(event `Persecucion`
  (params (Objetivo :type "Actor Object Reference"))
  ;[1 1 1] Persecución
  (set `self.EnCombate` true)
  (set `CharacterMovementComponent.MaxWalkSpeed` 500.0 (`self.CharacterMovement`))
  (`|AIMoveTo` self (0.0 0.0 0.0) Objetivo 80.0
    (:`OnSuccess`
      (`self.Golpe_Ataque`))
    (:`OnFail`
      _))
  (set `self.EnCombate` false)
  (set `CharacterMovementComponent.MaxWalkSpeed` 300.0 (`self.CharacterMovement`)))

(fn `UserConstructionScript`
  (`parent.UserConstructionScript`))