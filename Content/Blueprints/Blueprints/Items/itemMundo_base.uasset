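; Base world item pickup actor that the player collects by walking into it.
; On overlap with ThirdPersonCharacter it passes ElementoPickup to the character's ItemRecogido; if accepted, it plays a pickup sound at the collision component and destroys itself.
; Each tick it spins around its yaw axis and bobs vertically with a sine offset based on time since creation.
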(event `self.ReceiveBeginPlay`)

(event `self.ReceiveActorBeginOverlap`
  (params (OtherActor :type "Actor Object Reference"))
  (bind _asthird_person_character (cast `/Game/Blueprints/Blueprints/Personas/ThirdPersonCharacter` OtherActor))
  (bind _consumir (`/Game/Blueprints/Blueprints/Personas/ThirdPersonCharacter.Item_recogido` _asthird_person_character (`self.Elemento_pickup`)))
  (if _consumir
    (`GameplayStatics.PlaySoundAtLocation` (`self.Sonido_recoger`) (`SceneComponent.K2_GetComponentLocation` (`self.Colisión`)) (struct) 1.0 1.0 0.0 null null null)
    (`self.K2_DestroyActor`)))

(event `self.ReceiveTick`
  (params (DeltaSeconds :type "Float (single-precision)"))
  (`self.K2_AddActorLocalRotation` (* (`KismetMathLibrary.MakeRotator` 0.0 0.0 (`self.velocidad_rotacion`)) DeltaSeconds))
  (`self.K2_AddActorLocalOffset` (* (`KismetMathLibrary.Vector_Up`) (`KismetMathLibrary.DegSin` (* (`self.GetGameTimeSinceCreation`) (`self.velocidad_desplazo`))))))

(fn `UserConstructionScript`)