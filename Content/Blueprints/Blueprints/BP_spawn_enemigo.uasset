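; BP_spawn_enemigo is a placed spawn point that creates one enemy, either a melee or rifle type.
; On BeginPlay it binds to the ThirdPersonGameMode enemy-initialization event, which broadcasts a tag.
; When the tag matches TagEnemigo and its object name is absent from EnemigosMuertos, it spawns the chosen class at its transform.
; The enemy receives the spawner's name as IdActor, so killed enemies are not respawned.
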(event `self.ReceiveBeginPlay`
  (bind _asthird_person_game_mode (cast `/Game/Blueprints/Blueprints/Datos_juego/ThirdPersonGameMode` (`GameplayStatics.GetGameMode`)))
  (add `/Game/Blueprints/Blueprints/Datos_juego/ThirdPersonGameMode.Inicializar_enemigos_tag` _asthird_person_game_mode (delegate `delegate_crear_enemigo`)))

(event `delegate_crear_enemigo`
  (params (tag :type Integer))
  (bind _asthird_person_game_mode (cast `/Game/Blueprints/Blueprints/Datos_juego/ThirdPersonGameMode` (`GameplayStatics.GetGameMode`)))
  (if (and (== tag (`self.tag_enemigo`)) (not (`KismetArrayLibrary.Array_Contains` (`/Game/Blueprints/Blueprints/Datos_juego/ThirdPersonGameMode.Enemigos_muertos` _asthird_person_game_mode) (`KismetSystemLibrary.GetObjectName` self))))
    (`self.Crear_enemigo`)))

(fn `Crear_enemigo`
  (locals (clase_enemigo :type "/Game/Blueprints/Blueprints/Personas/BP_guardable Class Reference"))
  (`|ExecutionSequence`
    (:`then_0`
      (switch `/Game/Blueprints/Blueprints/enum_tipos_enemigo` (`self.tipo_enemigo`)
        (:`NewEnumerator0`
          (set `local.clase_enemigo` "/Game/Blueprints/Blueprints/Personas/BP_Enemigo_Golpes.BP_Enemigo_Golpes_C"))
        (:`NewEnumerator1`
          (set `local.clase_enemigo` "/Game/Blueprints/Blueprints/Personas/BP_Enemigo_Arma.BP_Enemigo_Arma_C"))))
    (:`then_1`
      (bind _returnvalue (`|SpawnActorFromClass` (`local.clase_enemigo`) (`self.GetTransform`) "Undefined" "OverrideRootScale" null null))
      (set `/Game/Blueprints/Blueprints/Personas/BP_guardable.id_actor` (`KismetSystemLibrary.GetObjectName` self) _returnvalue))))

(fn `UserConstructionScript`)