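; BP_Persona is a combat character with health, death, and punch, knife and rifle attacks.
; All attacks feed Atacar, a sphere trace applying damage and impact effects, with an Atacando cooldown.
; The rifle traces from the camera, pushed forward to gun distance, or along capsule-plus-offset aim without one.
; It also handles magazine reloading, weapon switching, and death by disabling collision, unpossessing and delayed destruction.
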(event `self.ReceiveAnyDamage`
  (params (Damage :type "Float (single-precision)") (DamageType :type "DamageType Object Reference") (InstigatedBy :type "Controller Object Reference") (DamageCauser :type "Actor Object Reference"))
  (bind _capsulecomponent (`self.CapsuleComponent`))
  ;[1 1 1] Daño
  (if (not (`self.Muerto`))
    (bind _output_get (set `self.Vida` (- (`self.Vida`) Damage)))
    (bind _output_get_2 (set `self.Muerto` (<= _output_get 0.0)))
    (`self.PlayAnimMontage` "/Game/MisModelos/Anmaciones/AM_daño.AM_daño")
    (if _output_get_2
      (`PrimitiveComponent.SetCollisionResponseToChannel` _capsulecomponent "ECC_Visibility" "ECR_Ignore")
      (`PrimitiveComponent.SetCollisionResponseToChannel` _capsulecomponent "ECC_Pawn" "ECR_Ignore")
      (`Controller.UnPossess` (`self.GetController`))
      (`KismetSystemLibrary.Delay` 10.0)
      (`self.K2_DestroyActor`))))

(event `Atacar`
  (params (`daño` :type "Float (double-precision)") (radio :type "Float (double-precision)") (Pos_inicial :type "Vector Structure") (Pos_final :type "Vector Structure") (duracion :type "Float (double-precision)") (Sonido_impacto :type "SoundBase Object Reference"))
  ;[1 1 1] Logica de Ataque
  (set `self.Atacando` true)
  (bind _outhit (`KismetSystemLibrary.SphereTraceSingle` Pos_inicial Pos_final radio "TraceTypeQuery1" false (`|MakeArray` self :!type "Actor Object Reference")))
  (bind (_bblockinghit _binitialoverlap _time _distance _location _impactpoint _normal _impactnormal _physmat _hitactor _hitcomponent) (`GameplayStatics.BreakHitResult` _outhit))
  (`/Engine/EditorBlueprintResources/StandardMacros.IsValid` _hitactor
    (:`Is Valid`
      (`GameplayStatics.ApplyDamage` _hitactor `daño`)
      (`GameplayStatics.PlaySoundAtLocation` Sonido_impacto _impactpoint (struct) 1.0 1.0 0.0 null null null)
      (`GameplayStatics.SpawnEmitterAtLocation` "/Game/Efectos/Effects/FX_Monsters/FX_Monster_Troll/death/P_TrollDeathImpact.P_TrollDeathImpact" _impactpoint (struct) (0.2 0.2 0.2) true "AutoRelease")
      (bind _returnvalue (`GameplayStatics.SpawnDecalAttached` "/Game/Extras/Mat_agujero.Mat_agujero" (5.0 5.0 5.0) _hitcomponent "None" _impactpoint (`KismetMathLibrary.Conv_VectorToRotator` _impactnormal) "KeepWorldPosition" 5.0))
      (`DecalComponent.SetFadeScreenSize` _returnvalue 0.0))
    (:`Is Not Valid`
      _))
  (`KismetSystemLibrary.Delay` duracion)
  (set `self.Atacando` false))

(event `Golpe_Ataque`
  (bind _outlocation (`self.GetActorEyesViewPoint`))
  ;[0.3906 0.3906 0.3906] Puñetazo
  (if (not (`self.Atacando`))
    (`self.PlayAnimMontage` "/Game/MisModelos/Anmaciones/AM_golpear.AM_golpear")
    (`self.Atacar` (`self.Daño_puño`) (`self.Radio_puño`) _outlocation (+ _outlocation (* (`KismetMathLibrary.GetForwardVector` (`self.Get absolute aim`)) (`self.Distancia_puño`))) 0.4 "/Game/Sonido/Golpe.Golpe")))

(event `Ataque_rifle_munición`
  (params (`Cámara` :type "CameraComponent Object Reference"))
  ;[1 1 1] Validación de munición
  (if (`self.Atacando`)
    _
    (elif (> (`self.Municion_cargador`) 0)
      (`/Engine/EditorBlueprintResources/StandardMacros.DecrementInt` (`self.Municion_cargador`)
        (:`  `
          (`self.Ataque Rifle` `Cámara`)))
      (else
        (`GameplayStatics.SpawnSoundAttached` "/Game/Sonido/wavs/rifle-clip-empty.rifle-clip-empty" (`self.SK_KA47`) "Muzzle" (0.0 0.0 0.0) (struct) "KeepRelativeOffset" false 1.0 1.0 0.0 null null)))))

(event `Recargar`
  (bind `_munición_reserva` (`self.Munición_reserva`))
  (bind _returnvalue (- (`self.Capacidad_cargador`) (`self.Municion_cargador`)))
  ;[1 1 1] Lógica recarga
  (if (>= `_munición_reserva` _returnvalue)
    (set `self.Munición_reserva` (- `_munición_reserva` _returnvalue))
    (set `self.Municion_cargador` (`self.Capacidad_cargador`))
    (else
      (set `self.Municion_cargador` (`self.Munición_reserva`))
      (set `self.Munición_reserva` 0))))

(event `Cuchillazo`
  (bind _outlocation (`self.GetActorEyesViewPoint`))
  ;[0.3906 0.3906 0.3906] Cuchillazo
  (if (not (`self.Atacando`))
    (`self.PlayAnimMontage` "/Game/MisModelos/Anmaciones/AM_Cuchillo.AM_Cuchillo")
    (`self.Atacar` (`self.Daño_cuchillo`) (`self.Radio_cuchillo`) _outlocation (+ _outlocation (* (`KismetMathLibrary.GetForwardVector` (`self.Get absolute aim`)) (`self.Distancia_cuchillo`))) 0.3 "/Game/Sonido/apuñalado_Cue.apuñalado_Cue")))

(event `Cambiar_arma`
  (params (Arma_actual :type "/Game/Blueprints/Blueprints/enum_forma_ataque Enum" :default "NewEnumerator0") (Nueva_arma :type "/Game/Blueprints/Blueprints/enum_forma_ataque Enum" :default "NewEnumerator0"))
  ;[1 1 1] Cambio de arma
  (`|ExecutionSequence`
    (:`then_0`
      (switch `/Game/Blueprints/Blueprints/enum_forma_ataque` Arma_actual
        (:`NewEnumerator1`
          (`self.PlayAnimMontage` "/Game/MisModelos/Anmaciones/AM_Guardar_rifle.AM_Guardar_rifle")
          (`SceneComponent.SetVisibility` (`self.SK_KA47`) false true))
        (:`NewEnumerator2`
          (`SceneComponent.SetVisibility` (`self.SK_M9_Knife`) false true)
          (`GameplayStatics.SpawnSoundAtLocation` "/Game/Sonido/sacar_cuchillo_Cue.sacar_cuchillo_Cue" (`self.K2_GetActorLocation`) (struct) 0.4 1.0 0.0 null null))))
    (:`then_1`
      (bind _output_get (set `self.Arma` Nueva_arma))
      (switch `/Game/Blueprints/Blueprints/enum_forma_ataque` _output_get
        (:`NewEnumerator1`
          (`self.PlayAnimMontage` "/Game/MisModelos/Anmaciones/AM_Agarrar_rifle.AM_Agarrar_rifle")
          (`SceneComponent.SetVisibility` (`self.SK_KA47`) true true))
        (:`NewEnumerator2`
          (`SceneComponent.SetVisibility` (`self.SK_M9_Knife`) true true)
          (`GameplayStatics.SpawnSoundAtLocation` "/Game/Sonido/sacar_cuchillo_Cue.sacar_cuchillo_Cue" (`self.K2_GetActorLocation`) (struct) 1.0 1.0 0.0 null null))))))

(fn `Ataque Rifle`
  (params (`Cámara` :type "CameraComponent Object Reference"))
  (locals (pos_inicio :type "Vector Structure") (pos_fin :type "Vector Structure"))
  (bind _returnvalue (`SceneComponent.K2_GetComponentLocation` `Cámara`))
  (bind _returnvalue_2 (`SceneComponent.GetForwardVector` `Cámara`))
  (if (not (`self.Atacando`))
    (`/Engine/EditorBlueprintResources/StandardMacros.IsValid` `Cámara`
      (:`Is Valid`
        (bind _output_get (set `local.pos_inicio` (+ (* _returnvalue_2 (`KismetMathLibrary.Vector_Distance` _returnvalue (`SceneComponent.K2_GetComponentLocation` (`self.SK_KA47`)))) _returnvalue)))
        (set `local.pos_fin` (+ (* _returnvalue_2 (`self.Distancia_rifle`)) _output_get)))
      (:`Is Not Valid`
        (bind _output_get_2 (set `local.pos_inicio` (`SceneComponent.K2_GetComponentLocation` (`self.CapsuleComponent`))))
        (set `local.pos_fin` (+ _output_get_2 (* (`KismetMathLibrary.GreaterGreater_VectorRotator` (1.0 0.0 0.0) (`self.Get absolute aim`)) (`self.Distancia_rifle`))))))
    (`self.PlayAnimMontage` "/Game/MisModelos/Anmaciones/AM_disparar.AM_disparar")
    (`GameplayStatics.SpawnEmitterAttached` "/Game/Efectos/Effects/FX_Monsters/FX_Monster_Gruntling/Master/P_BackPack_MuzzleFlash.P_BackPack_MuzzleFlash" (`self.SK_KA47`) "Muzzle" (0.0 0.0 0.0) (struct) (0.05 0.05 0.05) "KeepRelativeOffset" true "AutoRelease")
    (`self.Atacar` (`self.Daño_rifle`) (`self.Radio_bala_rifle`) (`local.pos_inicio`) (`local.pos_fin`) 0.1 "/Game/Sonido/Rifle/Impacto_bala.Impacto_bala")))

(fn `Get absolute aim`
  (returns (`rotacion_puntería` :type "Rotator Structure"))
  (bind (_apuntar_offset_roll _apuntar_offset_pitch _apuntar_offset_yaw) (`KismetMathLibrary.BreakRotator` (`self.apuntar_offset`)))
  (bind (_returnvalue_roll _returnvalue_pitch _returnvalue_yaw) (`KismetMathLibrary.BreakRotator` (`SceneComponent.K2_GetComponentRotation` (`self.CapsuleComponent`))))
  (return (`KismetMathLibrary.MakeRotator` (+ _returnvalue_roll _apuntar_offset_roll) (+ _returnvalue_pitch _apuntar_offset_pitch) (+ _returnvalue_yaw _apuntar_offset_yaw))))

(fn `Set absolute aim`
  (params (`Nueva dirección` :type "Rotator Structure"))
  (`self.K2_SetActorRotation` (`KismetMathLibrary.MakeRotator` 0.0 0.0 `Nueva dirección_Yaw`))
  (set `self.apuntar_offset` (`KismetMathLibrary.MakeRotator` 0.0 `Nueva dirección_Pitch`)))

(fn `UserConstructionScript`)